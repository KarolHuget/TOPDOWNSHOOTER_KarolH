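; BP_powerUp is a health pickup for the Marine_BP character.
; When Marine_BP overlaps its collision sphere, it adds Heal to Health without clamping, or prints a message if Health is already at least 100.
; It destroys itself in both cases.
; A timer using PowerUpDuration is set on every overlap before the cast, but names no function.
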(event `self.sphere collision.OnComponentBeginOverlap`
  (params (OverlappedComponent :type "PrimitiveComponent Object Reference") (OtherActor :type "Actor Object Reference") (OtherComp :type "PrimitiveComponent Object Reference") (OtherBodyIndex :type Integer) (bFromSweep :type Boolean) (SweepResult :type "HitResult Structure (by ref)"))
  (`KismetSystemLibrary.K2_SetTimer` null "" (`self.powerUp_duration`))
  (bind _asmarine_bp (cast `/Game/Marine_BP` OtherActor))
  (bind _health (`/Game/Marine_BP.health` _asmarine_bp))
  (if (>= _health 100.0)
    (`KismetSystemLibrary.PrintString` "Upsi Full health")
    (else
      (set `/Game/Marine_BP.health` (+ _health (`self.heal`)) _asmarine_bp)))
  (`self.K2_DestroyActor`))

(fn `UserConstructionScript`)
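; Player marine character with movement, mouse look, automatic rifle fire, health and death, plus a UI widget created on BeginPlay.
; Each tick, control rotation interpolates toward the direction of mouse velocity when it exceeds a dead zone, alongside sensitivity-scaled look inputs.
; Holding fire runs muzzle effects, sound and a looping timed line trace that applies damage along control rotation.
; Damage reduces clamped health; reaching zero stops firing effects and blocks player actions.
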(event `InputAxis|move_forward/back`
  (params (AxisValue :type "Float (single-precision)"))
  ;[0.8463 1 0.5003] Walking
  (if (`self.is_alive`)
    (`self.AddMovementInput` (`SceneComponent.GetForwardVector` (`self.CapsuleComponent`)) (* AxisValue (`self.movement_multiplayer`)))))

(event `InputAxis|move_left/right`
  (params (AxisValue :type "Float (single-precision)"))
  ;[0.8463 1 0.5003] Walking
  (if (`self.is_alive`)
    (`self.AddMovementInput` (`SceneComponent.GetRightVector` (`self.CapsuleComponent`)) (* AxisValue (`self.movement_multiplayer`)))))

(event `self.ReceiveTick`
  (params (DeltaSeconds :type "Float (single-precision)"))
  ;[0.2825 0.3984 1] rotation
  (if (`self.is_alive`)
    (`self.update_player_rotation`)))

(event `self.ReceiveBeginPlay`
  ;[0.03036 1 0.3644] UI
  (bind _returnvalue (`|CreateWidget` "/Game/UIwidget.UIwidget_C" null self))
  (`UserWidget.AddToViewport` _returnvalue 0))

(event `InputAction|fire_weapon`
  (params (Key :type "Key Structure"))
  ;[0.08854 0.03459 0.03459] Shooting
  (:`Pressed`
    (if (`self.is_alive`)
      (`self.start_firing`)
      (`self.weaponTrace`)
      (`KismetSystemLibrary.K2_SetTimer` null "weaponTrace" 0.18 true)
      (else
        (`self.Stop Firing` :!label _label)
        (`KismetSystemLibrary.K2_ClearTimer` null "weaponTrace"))))
  (:`Released`
    (goto _label)))

(event `InputAxis|LookUp`
  (params (AxisValue :type "Float (single-precision)"))
  ;[1 0.3704 0.906] camera_sensitiviti
  (if (`self.is_alive`)
    (`self.AddControllerPitchInput` (* AxisValue (`self.mouse_sensitivity`)))))

(event `InputAxis|Turn`
  (params (AxisValue :type "Float (single-precision)"))
  ;[1 0.3704 0.906] camera_sensitiviti
  (if (`self.is_alive`)
    (`self.AddControllerYawInput` (* AxisValue (`self.mouse_sensitivity`)))))

(event `self.ReceiveAnyDamage`
  (params (Damage :type "Float (single-precision)") (DamageType :type "DamageType Object Reference") (InstigatedBy :type "Controller Object Reference") (DamageCauser :type "Actor Object Reference"))
  ;[0.7083 0.7083 0.7083] Death
  (bind _output_get (set `self.health` (`KismetMathLibrary.FClamp` (- (`self.health`) Damage) 0.0 100.0)))
  (bind _output_get_2 (set `self.is_dead` (== _output_get 0.0)))
  (if _output_get_2
    (`self.Stop Firing`)))

(fn `get_mouse_velocity`
  (returns (ReturnValue :type "Vector2D Structure"))
  (bind (_deltax _deltay) (`PlayerController.GetInputMouseDelta` (`GameplayStatics.GetPlayerController` 0)))
  (return (/ (`KismetMathLibrary.MakeVector2D` _deltax _deltay) (`GameplayStatics.GetWorldDeltaSeconds`))))

(fn `getENDlocationLT`
  (returns (ReturnValue :type "Vector Structure"))
  (return (+ (`self.GetSTARTocationLT`) (* (`KismetMathLibrary.GetForwardVector` (`self.GetControlRotation`)) (`self.weaponRange`)))))

(fn `GetSTARTocationLT`
  (returns (ReturnValue :type "Vector Structure"))
  (return (`SceneComponent.GetSocketLocation` (`self.SkeletalMesh`) "None")))

(fn `is_alive`
  (returns (ReturnValue :type Boolean))
  (return (not (`self.is_dead`))))

(fn `Mouse above DeadZone`
  (returns (ReturnValue :type Boolean))
  (return (> (`KismetMathLibrary.VSize2D` (`self.get_mouse_velocity`)) (`self.DeadZone`))))

(fn `start_firing`
  (if (`self.is_alive`)
    (`ActorComponent.Activate` (`self.P_AssaultRifle_MF`) false)
    (bind _returnvalue (`GameplayStatics.SpawnSound2D` "/Game/Sounds/randomfiresound.randomfiresound" 1.0 1.0 0.0 null))
    (set `self.firesound1` _returnvalue)))

(fn `Stop Firing`
  (bind _firesound1 (`self.firesound1`))
  (`ActorComponent.Deactivate` (`self.P_AssaultRifle_MF`))
  (`/Engine/EditorBlueprintResources/StandardMacros.IsValid` _firesound1
    (:`Is Valid`
      (`AudioComponent.Stop` _firesound1)
      (if (`self.is_alive`)
        (bind _returnvalue (`GameplayStatics.SpawnSound2D` "/Game/Sounds/fireendsound.fireendsound" 1.0 1.0 0.0 null))
        (set `self.soundend1` _returnvalue)))))

(fn `update_player_rotation`
  (bind (_returnvalue_x _returnvalue_y) (`KismetMathLibrary.BreakVector2D` (`self.get_mouse_velocity`)))
  (bind _returnvalue (`GameplayStatics.GetPlayerController` 0))
  (if (`self.is_alive`)
    (if (`self.Mouse above DeadZone`)
      (`Controller.SetControlRotation` _returnvalue (`KismetMathLibrary.RInterpTo` (`Controller.GetControlRotation` _returnvalue) (`KismetMathLibrary.MakeRotator` 0.0 0.0 (`KismetMathLibrary.DegAtan2` _returnvalue_x _returnvalue_y)) (`GameplayStatics.GetWorldDeltaSeconds`) (`self.delta_time_multiply`))))))

(fn `UserConstructionScript`)

(fn `weaponTrace`
  (bind _outhit (`KismetSystemLibrary.LineTraceSingle` :`Start` (`self.GetSTARTocationLT`) :`End` (`self.getENDlocationLT`) :`TraceChannel` "TraceTypeQuery1" :`DrawDebugType` "ForDuration"))
  (`GameplayStatics.ApplyDamage` (`.HitActor` (`GameplayStatics.BreakHitResult` _outhit)) (`self.FireDamage`)))